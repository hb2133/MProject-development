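; Construction-script Blueprint that displays an array of materials on a grid of generated spheres, one material per sphere.
; It derives a near-square grid size from the square root of the material count and centres the grid on the actor using the Distance spacing.
; Nested loops add a static mesh component at each cell, assign the next material, and break once the list runs out to avoid redundant spheres.
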(fn ConstructionScript
  (bind _materialarrayindex (LocalVariables|GetMaterialArrayIndex))
  ;[1 1 1] get array size X*Y
  (bind _output_get (LocalVariables|SetSQRT (Math|Float|Sqrt (Math|Conversions|ToFloat(Integer) (Utilities|Array|Length (Variables|Default|Getmaterials))))))
  (LocalVariables|SetLastIndexX (- (Math|Float|Ceil _output_get) 1))
  (LocalVariables|SetLastIndexY (- (Math|Float|Round (LocalVariables|GetSQRT)) 1))
  ;[1 1 1] center the array
  (LocalVariables|Setoffset (/ (Math|Vector|MakeVector (CallFunction|MultiplyDistance (LocalVariables|GetLastIndexX)) (CallFunction|MultiplyDistance (LocalVariables|GetLastIndexY)) 0.0) -2))
  ;[1 1 1] line X
  (for _index (range 0 (LocalVariables|GetLastIndexX))
    (LocalVariables|SetdistanceX (CallFunction|MultiplyDistance _index))
    ;[1 1 1] line Y
    (bind _index_2 (Utilities|FlowControl|ForLoopwithBreak 0 (LocalVariables|GetLastIndexY) :!label _label)
      (:LoopBody
        (LocalVariables|SetindexY _index_2)
        (Utilities|FlowControl|Sequence
          (:then_0
            ;[1 1 1] place spheres with materials
            (bind _returnvalue (AddComponent|AddStaticMeshComponent false (Math|Transform|MakeTransform (+ (Math|Vector|MakeVector (LocalVariables|GetdistanceX) (CallFunction|MultiplyDistance (LocalVariables|GetindexY)) 0.0) (LocalVariables|Getoffset)) "0, 0, 0" "1.000000,1.000000,1.000000")))
            (Rendering|Material|SetMaterial _returnvalue 0 (Utilities|Array|Get(acopy) (Variables|Default|Getmaterials) (LocalVariables|GetMaterialArrayIndex))))
          (:then_1
            ;[1 1 1] prevent placing redundant spheres
            (Math|Integer|IncrementInt _materialarrayindex
              (:%20%20
                (if (> _materialarrayindex (Utilities|Array|LastIndex (Variables|Default|Getmaterials)))
                  (goto _label Break))))))))))

(fn MultiplyDistance
  (params (A :type Integer%20%28by%20ref%29))
  (return (* A (Variables|Default|Getdistance))))